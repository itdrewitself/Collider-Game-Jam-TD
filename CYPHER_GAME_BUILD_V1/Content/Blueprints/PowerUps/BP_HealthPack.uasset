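; BP_HealthPack is a health pickup that spins and bobs on a timeline around a fixed world height.
; Any overlap on its Box adds HealthPackSM to player 0's BP_Hero health, clamped to one, without checking which actor overlapped.
; If health is not already full, the pack destroys itself and pushes the new value to the hero's WBP_Healthbar widget.
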(event `self.ReceiveTick`
  (params (DeltaSeconds :type "Float (single-precision)"))
  (bind _box (`self.Box`))
  (bind (_returnvalue_x _returnvalue_y) (`KismetMathLibrary.BreakVector` (`SceneComponent.K2_GetComponentLocation` (`self.Box`))))
  ;[1 1 1] Bounce
  (`/Engine/EditorBlueprintResources/StandardMacros.IsValid` _box
    (:`Is Valid`
      (`SceneComponent.K2_AddLocalRotation` _box (`KismetMathLibrary.MakeRotator` 0.0 0.0 1.0) false false)
      (bind (_direction _newtrack_2) (`Timeline|Bounce`)
        (:`Update`
          (`self.K2_SetActorLocation` (`KismetMathLibrary.MakeVector` _returnvalue_x _returnvalue_y (+ (* _newtrack_2 50.0) 80.0))))))))

(event `self.Box.OnComponentBeginOverlap`
  (params (OverlappedComponent :type "PrimitiveComponent Object Reference") (OtherActor :type "Actor Object Reference") (OtherComp :type "PrimitiveComponent Object Reference") (OtherBodyIndex :type Integer) (bFromSweep :type Boolean) (SweepResult :type "HitResult Structure (by ref)"))
  ;[1 1 1] Health
  ;;[1 1 1] Cast to Player
  (bind _asbp_hero (cast `/Game/Blueprints/Hero/BP_Hero` (`GameplayStatics.GetPlayerCharacter` 0)))
  (bind _playerhealth (`/Game/Blueprints/Hero/BP_Hero.PlayerHealth` _asbp_hero))
  ;;[1 1 1] Check Full health
  (if (!= _playerhealth 1.0)
    ;;[1 1 1] Apply Health
    (bind _output_get (set `/Game/Blueprints/Hero/BP_Hero.PlayerHealth` (`KismetMathLibrary.FClamp` (+ _playerhealth (`self.HealthPackSM`))) _asbp_hero))
    ;;[1 1 1] Destroy Health box
    (`self.K2_DestroyActor` self)
    ;;[1 1 1] Update Healthbar
    (bind _aswbp_healthbar (cast `/Game/Blueprints/UI/WBP_Healthbar` (`WidgetComponent.GetWidget` (`/Game/Blueprints/Hero/BP_Hero.HealthBar` _asbp_hero))))
    (`/Game/Blueprints/UI/WBP_Healthbar.Update Health` _aswbp_healthbar _output_get)))

(fn `UserConstructionScript`)