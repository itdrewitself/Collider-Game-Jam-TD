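; BP_Director is the zombie horde director that tracks every BP_Horde zombie and governs spawning up to a maximum population.
; On BeginPlay it registers existing zombies and BP_HordeSpawner actors, binding to their killed and spawn request events.
; Spawn requests create zombies at random reachable navmesh points around the requested location, capped by remaining slots under MaxZombies.
; New zombies are registered, and killed ones leave the list, freeing slots.
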(event `self.ReceiveBeginPlay`
  (`|ExecutionSequence`
    (:`then_0`
      (bind _outactors (`GameplayStatics.GetAllActorsOfClass` "/Game/Blueprints/Zombie/BP_Horde.BP_Horde_C"))
      (for _array_element _outactors
        (`self.On Zombie Spawn` _array_element)))
    (:`then_1`
      (bind _outactors_2 (`GameplayStatics.GetAllActorsOfClass` "/Game/Blueprints/Framework/BP_HordeSpawner.BP_HordeSpawner_C"))
      (for _array_element_2 _outactors_2
        (`self.OnHordeSpawnerSpawn` _array_element_2)))))

(fn `On Zombie Killed`
  (params (`Horde Zombie` :type "/Game/Blueprints/Zombie/BP_Horde Object Reference"))
  (`KismetArrayLibrary.Array_RemoveItem` (`self.Zombies`) `Horde Zombie`))

(fn `On Zombie Spawn`
  (params (`Horde Zombie` :type "/Game/Blueprints/Zombie/BP_Horde Object Reference"))
  (`KismetArrayLibrary.Array_Add` (`self.Zombies`) `Horde Zombie`)
  (`/Engine/EditorBlueprintResources/StandardMacros.IsValid` `Horde Zombie`
    (:`Is Valid`
      (add `/Game/Blueprints/Zombie/BP_Horde.OnKilled` `Horde Zombie` (`|CreateDelegate` :!event `On Zombie Killed`)))))

(fn `OnHordeSpawnerSpawn`
  (params (`Horde Spawner` :type "/Game/Blueprints/Framework/BP_HordeSpawner Object Reference"))
  (`KismetArrayLibrary.Array_Add` (`self.Horde Spawners`) `Horde Spawner`)
  (add `/Game/Blueprints/Framework/BP_HordeSpawner.RequestSpawn` `Horde Spawner` (`|CreateDelegate` :!event `OnZombiSpawnRequested`)))

(fn `OnZombiSpawnRequested`
  (params (Count :type Integer) (Location :type "Vector Structure"))
  (for _ (range 1 (+ (`KismetMathLibrary.Min` Count (- (`self.Max Zombies`) (`KismetArrayLibrary.Array_Length` (`self.Zombies`)))) 1))
    (bind _returnvalue (`|SpawnActorFromClass` "/Game/Blueprints/Zombie/BP_Horde.BP_Horde_C" (`KismetMathLibrary.MakeTransform` (+ (`NavigationSystemV1.K2_GetRandomReachablePointInRadius` (`local.Location`) 0.0 null null) (0.0 0.0 88.0))) "AdjustIfPossibleButDontSpawnIfColliding" "OverrideRootScale" null null))
    (`/Engine/EditorBlueprintResources/StandardMacros.IsValid` _returnvalue
      (:`Is Valid`
        (`self.On Zombie Spawn` _returnvalue)))))

(fn `UserConstructionScript`)