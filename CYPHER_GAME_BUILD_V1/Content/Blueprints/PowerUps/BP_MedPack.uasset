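; BP_MedPack is a health pickup that spins and bobs until collected.
; Tick rotates the Box and plays a timeline that sets the actor's world Z absolutely, ignoring placed height.
; Any Box overlap, without checking the overlapping actor, heals player 0's BP_Hero by a quarter, capped at full, unless already full.
; Healing updates the WBP_Healthbar widget, destroys the pack and spawns a heal particle at the player.
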(event `self.ReceiveBeginPlay`)

(event `self.ReceiveTick`
  (params (DeltaSeconds :type "Float (single-precision)"))
  (bind _box (`self.Box`))
  (bind _box_2 (`self.Box`))
  (bind (_returnvalue_x _returnvalue_y) (`KismetMathLibrary.BreakVector` (`SceneComponent.K2_GetComponentLocation` _box)))
  ;[1 1 1] Bounce
  (`SceneComponent.K2_AddLocalRotation` _box_2 (`KismetMathLibrary.MakeRotator` 0.0 0.0 1.0) false false)
  (`/Engine/EditorBlueprintResources/StandardMacros.IsValid` _box_2
    (:`Is Valid`
      (bind (_direction _newtrack_2) (`Timeline|Timeline_0`)
        (:`Update`
          (`/Engine/EditorBlueprintResources/StandardMacros.IsValid` _box
            (:`Is Valid`
              (`self.K2_SetActorLocation` (`KismetMathLibrary.MakeVector` _returnvalue_x _returnvalue_y (* _newtrack_2 50.0))))))))))

(event `self.Box.OnComponentBeginOverlap`
  (params (OverlappedComponent :type "PrimitiveComponent Object Reference") (OtherActor :type "Actor Object Reference") (OtherComp :type "PrimitiveComponent Object Reference") (OtherBodyIndex :type Integer) (bFromSweep :type Boolean) (SweepResult :type "HitResult Structure (by ref)"))
  (bind _returnvalue (`GameplayStatics.GetPlayerCharacter` 0))
  ;[1 1 1] Add Health
  (`/Engine/EditorBlueprintResources/StandardMacros.IsValid` _returnvalue
    (:`Is Valid`
      (bind _asbp_hero (cast `/Game/Blueprints/Hero/BP_Hero` _returnvalue))
      (`|ExecutionSequence`
        (:`then_0`
          (bind _playerhealth (`/Game/Blueprints/Hero/BP_Hero.PlayerHealth` _asbp_hero))
          (if (!= _playerhealth 1.0)
            (bind _output_get (set `/Game/Blueprints/Hero/BP_Hero.PlayerHealth` (`KismetMathLibrary.FClamp` (+ _playerhealth 0.25)) _asbp_hero))
            (bind _aswbp_healthbar (cast `/Game/Blueprints/UI/WBP_Healthbar` (`WidgetComponent.GetWidget` (`/Game/Blueprints/Hero/BP_Hero.HealthBar` _asbp_hero))))
            (`/Game/Blueprints/UI/WBP_Healthbar.Update Health` _aswbp_healthbar _output_get)
            (`self.K2_DestroyActor`)
            (`GameplayStatics.SpawnEmitterAtLocation` "/Game/VFX/InfinityBladeEffects/Effects/FX_Ability/Heal/P_Heal_Startup_mobile.P_Heal_Startup_mobile" (`self.K2_GetActorLocation` _returnvalue) (struct) (1.5 1.5 1.5))))
        (:`then_1`)))))

(fn `UserConstructionScript`)