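; BP_HordeSpawner is a trigger-based spawner that requests a horde of enemies when a hero walks into it.
; On overlap with a BP_Hero tagged "hero", it calls a spawn request with a random count between its min and max horde size at the SpawnLocation component.
; It then sets the trigger box to no collision, and a timer restores it after a fixed cooldown so it can fire again.
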(event `self.TriggerBox.OnComponentBeginOverlap`
  (params (OverlappedComponent :type "PrimitiveComponent Object Reference") (OtherActor :type "Actor Object Reference") (OtherComp :type "PrimitiveComponent Object Reference") (OtherBodyIndex :type Integer) (bFromSweep :type Boolean) (SweepResult :type "HitResult Structure (by ref)"))
  (bind _asbp_hero (cast `/Game/Blueprints/Hero/BP_Hero` OtherActor))
  (if (`self.ActorHasTag` _asbp_hero "hero")
    (`PrimitiveComponent.SetCollisionProfileName` (`self.TriggerBox`) "nocollision" true)
    (`KismetSystemLibrary.K2_SetTimerDelegate` (delegate `Enable Trigger`) 30.0)
    (`self.RequestSpawn` (`KismetMathLibrary.RandomIntegerInRange` (`self.Horde Size Min`) (`self.Horde Size Max`)) (`SceneComponent.K2_GetComponentLocation` (`self.Spawn Location`)))))

(event `Enable Trigger`
  (`PrimitiveComponent.SetCollisionProfileName` (`self.TriggerBox`) "Trigger" true))

(fn `UserConstructionScript`)