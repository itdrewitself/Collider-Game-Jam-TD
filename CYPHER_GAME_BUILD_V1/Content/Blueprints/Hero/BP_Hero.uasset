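; Player hero character with camera-relative movement, aim-gated shooting, HUD widgets and ragdoll death.
; Aiming slows movement, sets AGR aim offset and rotation, and enables firing if ammo remains.
; Firing spawns a delayed actor at the weapon's barrel socket and traces for blood effects on Enemy-tagged actors, while Tick draws a debug-shape crosshair.
; EnterDeathState shows the death screen, disables input, ragdolls the mesh and unregisters AI perception.
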(event `self.ReceiveBeginPlay`
  (`|ExecutionSequence`
    (:`then_0`
      ;[1 1 1] Kill Counter
      (bind _returnvalue (`|CreateWidget` "/Game/Blueprints/UI/WBP_Killcount.WBP_Killcount_C"))
      (`UserWidget.AddToViewport` _returnvalue 0))
    (:`then_1`
      (bind _aswbp_healthbar_hover (cast `/Game/Blueprints/UI/WBP_HealthbarHover` (`WidgetComponent.GetWidget` (`self.HealthBar`))))
      (`/Game/Blueprints/UI/WBP_HealthbarHover.Update Health` _aswbp_healthbar_hover (`self.PlayerHealth`)))
    (:`then_2`
      ;[1 0.3712 0.2502] Attach Weapon
      (`SceneComponent.K2_AttachToComponent` (`self.PrimaryWeapon`) (`self.Mesh`) "weapon_socket" "SnapToTarget" "SnapToTarget" "SnapToTarget" true))))

(event `InputAction|Aim`
  (params (Key :type "Key Structure"))
  ;[1 1 1] Aim?Walk
  (:`Pressed`
    (set `self.Walk` true))
  (:`Released`
    (set `self.Walk` false)))

(event `InputAxis|Move Forward / Backward`
  (params (AxisValue :type "Float (single-precision)"))
  (bind (_returnvalue_roll _returnvalue_pitch _returnvalue_yaw) (`KismetMathLibrary.BreakRotator` (`SceneComponent.K2_GetComponentRotation` (`self.Camera`))))
  ;[1 1 1] WASD
  (`self.AddMovementInput` (`KismetMathLibrary.GetForwardVector` (`KismetMathLibrary.MakeRotator` 0.0 0.0 _returnvalue_yaw)) (`KismetMathLibrary.SelectFloat` (/ AxisValue 3.0) AxisValue (`self.Walk`))))

(event `InputAxis|Turn Right / Left Mouse`
  (params (AxisValue :type "Float (single-precision)"))
  ;[1 1 1] Camera Movement
  (`self.AddControllerYawInput` AxisValue))

(event `InputAxis|Look Up / Down Mouse`
  (params (AxisValue :type "Float (single-precision)"))
  ;[1 1 1] Camera Movement
)

(event `InputAxis|Move Right / Left`
  (params (AxisValue :type "Float (single-precision)"))
  (bind (_returnvalue_roll _returnvalue_pitch _returnvalue_yaw) (`KismetMathLibrary.BreakRotator` (`SceneComponent.K2_GetComponentRotation` (`self.Camera`))))
  ;[1 1 1] WASD
  (`self.AddMovementInput` (`KismetMathLibrary.GetRightVector` (`KismetMathLibrary.MakeRotator` _returnvalue_roll 0.0 _returnvalue_yaw)) (`KismetMathLibrary.SelectFloat` (/ AxisValue 3.0) AxisValue (`self.Walk`))))

(event `InputAction|Aim`
  (params (Key :type "Key Structure"))
  (bind _agranimmaster (`self.AGRAnimMaster`))
  ;[1 1 1] Set Aim Type
  (:`Pressed`
    (`AGRAnimMasterComponent.SetupAimOffset` _agranimmaster "Aim" "Nearest" 90.0 false "hand_r" "head")
    (`AGRAnimMasterComponent.SetupRotation` _agranimmaster "AbsoluteRotation" 360.0 90.0 5.0))
  (:`Released`
    (`AGRAnimMasterComponent.SetupAimOffset` _agranimmaster "NONE" "Nearest" 90.0 false "hand_r" "head")
    (`AGRAnimMasterComponent.SetupRotation` _agranimmaster "AbsoluteRotation" 360.0 90.0 5.0)))

(event `InputAction|Fire`
  (params (Key :type "Key Structure"))
  ;[1 0.3712 0.2502] Full Auto
  (:`Pressed`
    (if (`self.CanFire`)
      (`KismetSystemLibrary.Delay` 0.15)
      (bind _return_value_location (`self.GetWeaponSocket` "BarrelSocket"))
      (`|SpawnActorFromClass` "/Game/Blueprints/Weapons/BP_AR4_Projectile.BP_AR4_Projectile_C" (`KismetMathLibrary.MakeTransform` (.location _return_value_location) (.rotation _return_value_location) (0.3 0.3 0.3)) "Undefined" "OverrideRootScale" null null))))

(event `InputAction|Aim`
  (params (Key :type "Key Structure"))
  ;[1 1 1] Check Can Fire
  ;;[1 1 1] Check Aiming
  (:`Pressed`
    ;;[1 1 1] Check Ammo
    (if (> (`self.Ammo`) 0)
      (set `self.CanFire` true)
      (`KismetSystemLibrary.Delay` 0.15)
      (else
        (set `self.CanFire` false)
        (set `self.IsFiring` false))))
  (:`Released`
    (set `self.CanFire` false)))

(event `InputAction|Fire`
  (params (Key :type "Key Structure"))
  ;[1 1 1] SHOOTING
  ;;[1 1 1] Blood Splatter
  (:`Pressed`
    (if (`self.CanFire`)
      (`self.GetWeaponSocket` "BarrelSocket")
      (bind _outhit (`KismetSystemLibrary.LineTraceSingle` (.location (stale `self.ReceiveTick` _return_value_location)) (+ (.location (stale `self.ReceiveTick` _return_value_location)) (* (`KismetMathLibrary.GetForwardVector` (.rotation (stale `self.ReceiveTick` _return_value_location))) 10000)) "TraceTypeQuery1"))
      (bind (_bblockinghit _binitialoverlap _time _distance _location _impactpoint _normal _impactnormal _physmat _hitactor) (`GameplayStatics.BreakHitResult` _outhit))
      (`/Engine/EditorBlueprintResources/StandardMacros.IsValid` _hitactor
        (:`Is Valid`
          (if (`self.ActorHasTag` _hitactor "Enemy")
            (`NiagaraFunctionLibrary.SpawnSystemAtLocation` "/Game/VFX/sA_SplatterofbloodFx/Fx/PreShaded_Blood_Alternatives/NS_PreShadedBlood_4.NS_PreShadedBlood_4" _impactpoint (struct) (2.0 2.0 2.0))))))))

(event `self.ReceiveTick`
  (params (DeltaSeconds :type "Float (single-precision)"))
  ;[1 1 1] SHOOTING
  ;;[1 1 1] Hit Crosshaier
  (`|ExecutionSequence`
    (:`then_0`
      (if (`self.CanFire`)
        (bind _return_value_location (`self.GetWeaponSocket` "BarrelSocket"))
        (bind _outhit (`KismetSystemLibrary.LineTraceSingle` (.location _return_value_location) (+ (.location _return_value_location) (* (`KismetMathLibrary.GetForwardVector` (.rotation _return_value_location)) 10000)) "TraceTypeQuery1"))))
    (:`then_1`
      ;;[0.147 1 0.5776] Crosshair
      (if (`self.CanFire`)
        (bind _return_value_location_2 (`self.GetWeaponSocket` "BarrelSocket"))
        (bind _outhit_2 (`KismetSystemLibrary.LineTraceSingle` (.location _return_value_location_2) (+ (.location _return_value_location_2) (* (`KismetMathLibrary.GetForwardVector` (.rotation _return_value_location_2)) 300)) "TraceTypeQuery1"))
        (`KismetSystemLibrary.DrawDebugBox` (`.TraceEnd` (`GameplayStatics.BreakHitResult` _outhit_2)) (15.0 0.0 15.0) (struct :`G` 1.0 :`B` 0.176207 :`A` 1.0) (`SceneComponent.K2_GetComponentRotation` (`self.PrimaryWeapon`)) 0.0 5.0)
        (bind (_bblockinghit _binitialoverlap _time _distance _location _impactpoint) (`GameplayStatics.BreakHitResult` _outhit))
        (if _bblockinghit
          (`KismetSystemLibrary.DrawDebugSphere` _impactpoint 30.0 12 (struct :`R` 1.0 :`B` 0.066577 :`A` 1.0)))))))

(fn `EnterDeathState`
  (bind _returnvalue (`GameplayStatics.GetPlayerController` 0))
  (bind _returnvalue_2 (`|CreateWidget` "/Game/Blueprints/UI/WBP_DeathScreen.WBP_DeathScreen_C" _returnvalue))
  (`UserWidget.AddToViewport` _returnvalue_2 0)
  (`self.DisableInput` _returnvalue)
  (set `self.IsDead` true)
  (`self.Ragdoll`)
  (`AIPerceptionStimuliSourceComponent.UnregisterFromPerceptionSystem` (`self.AIPerceptionStimuliSource`)))

(fn `GetWeaponSocket`
  (params (`Socket Name` :type Name))
  (returns (`Return Value Location` :type "Transform Structure"))
  (bind _primaryweapon (`self.PrimaryWeapon`))
  (`/Engine/EditorBlueprintResources/StandardMacros.IsValid` _primaryweapon
    (:`Is Valid`
      (return (`SceneComponent.GetSocketTransform` _primaryweapon `Socket Name` "RTS_World")))))

(fn `Ragdoll`
  (`PrimitiveComponent.SetSimulatePhysics` (`self.Mesh`) true))

(fn `UserConstructionScript`)