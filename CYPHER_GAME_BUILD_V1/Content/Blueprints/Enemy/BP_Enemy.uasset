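; BP_Enemy is an enemy character with health, a health bar widget and ragdoll death.
; On BeginPlay it initialises the EnemyHealthBar widget and passes its behavior tree to AI_EnemyController.
; Damage lowers Health and updates the bar.
; The death check runs before subtraction, so the ragdoll (mesh physics on, movement disabled) only triggers on a hit received when Health is already zero or below.
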(event `self.ReceiveBeginPlay`
  (`|ExecutionSequence`
    (:`then_0`
      ;[1 1 1] Initialise HealthBar
      (bind _asenemy_health_bar (cast `/Game/Blueprints/UI/EnemyHealthBar` (`WidgetComponent.GetUserWidgetObject` (`self.HealthBar`))))
      (bind _output_get (set `self.Enemy Health Widget` _asenemy_health_bar))
      (`/Game/Blueprints/UI/EnemyHealthBar.Update Health` _output_get (`self.Health`)))
    (:`then_1`
      ;[1 1 1] Initialise AI Type
      (bind _asai_controller_enemy (cast `/Game/Blueprints/Enemy/AI_EnemyController` (`AIBlueprintHelperLibrary.GetAIController` self)))
      (`/Game/Blueprints/Enemy/AI_EnemyController.Setup AIC` _asai_controller_enemy "/Game/Blueprints/Enemy/BT_Enemy.BT_Enemy"))))

(event `self.ReceiveAnyDamage`
  (params (Damage :type "Float (single-precision)") (DamageType :type "DamageType Object Reference") (InstigatedBy :type "Controller Object Reference") (DamageCauser :type "Actor Object Reference"))
  (bind _health (`self.Health`))
  ;[1 1 1] On damage
  (bind _output_get (set `self.IsDead` (<= _health 0.0)))
  (if _output_get
    (`self.Ragdoll`)
    (else
      (bind _output_get_2 (set `self.Health` (- _health Damage)))
      (`/Game/Blueprints/UI/EnemyHealthBar.Update Health` (`self.Enemy Health Widget`) _output_get_2))))

(event `Ragdoll`
  ;[1 1 1] Ragdoll
  (`PrimitiveComponent.SetSimulatePhysics` (`self.Mesh`) true)
  (`CharacterMovementComponent.DisableMovement` (`self.CharacterMovement`)))

(fn `UserConstructionScript`)